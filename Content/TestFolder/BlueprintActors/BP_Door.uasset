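; BP_Door is a door actor that swings open and closed by rotating around its yaw axis.
; OpenDoor and CloseDoor events set the sign of a yaw increment and raise a movement flag, skipping if the door is already at that limit.
; Tick then adds the increment each frame, independent of delta time, and clears the flag once world yaw reaches 90 degrees open or zero closed.
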(event Custom|OpenDoor
  (if (< (.yaw (Transformation|GetActorRotation)) 9e+01)
    (Variables|Default|SetYawIncrement 2.0)
    (Variables|Default|SetOpen_Close_Door true)))

(event Custom|CloseDoor
  (if (> (.yaw (Transformation|GetActorRotation)) 0.0)
    (Variables|Default|SetYawIncrement -2.0)
    (Variables|Default|SetOpen_Close_Door true)))

(event Collision|EventActorBeginOverlap
  (params (OtherActor :type Actor%20Object%20Reference)))

(event EventTick
  (params (DeltaSeconds :type Float%20%28single-precision%29))
  (bind _returnvalue (Transformation|GetActorRotation))
  (if (Variables|Default|GetOpen_Close_Door)
    (Transformation|SetActorRotation (Math|Rotator|MakeRotator (.roll _returnvalue) (.pitch _returnvalue) (+ (.yaw _returnvalue) (Variables|Default|GetYawIncrement))))
    (if (or (and (> (Variables|Default|GetYawIncrement) 0.0) (>= (.yaw (Transformation|GetActorRotation)) 9e+01)) (and (< (Variables|Default|GetYawIncrement) 0.0) (<= (.yaw (Transformation|GetActorRotation)) 0.0)))
      (Variables|Default|SetOpen_Close_Door false))))

(fn ConstructionScript)